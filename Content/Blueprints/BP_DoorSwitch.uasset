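; BP_DoorSwitch is a door switch actor whose mesh has red and green indicator lights showing whether it is locked or openable.
; On BeginPlay, IsLocked and IsOpenable independently select emissive or non-emissive materials for the red and green mesh slots.
; The lights are set only at startup, and the graph contains no interaction logic or later updates.
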(event `self.ReceiveBeginPlay`
  (`|ExecutionSequence`
    (:`then_0`
      (if (`self.IsLocked`)
        (`PrimitiveComponent.SetMaterial` (`self.Mesh`) 1 "/Game/Materials/MI_Light_Red.MI_Light_Red")
        (else
          (`PrimitiveComponent.SetMaterial` (`self.Mesh`) 1 "/Game/Materials/MI_Light_Red_NoEmmision.MI_Light_Red_NoEmmision"))))
    (:`then_1`
      (if (`self.IsOpenable`)
        (`PrimitiveComponent.SetMaterial` (`self.Mesh`) 2 "/Game/Materials/MI_Light_Green.MI_Light_Green")
        (else
          (`PrimitiveComponent.SetMaterial` (`self.Mesh`) 2 "/Game/Materials/MI_Light_Green_NoEmmision.MI_Light_Green_NoEmmision"))))))

(fn `UserConstructionScript`)